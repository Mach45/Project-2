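; Game instance that drives main menus, campaign starts, LAN/online session host and join, and error handling across level loads.
; A player-state machine removes the outgoing state's widget, while GIShowMainMenu lazily creates and swaps menu widgets.
; Player controller, player state and map register after each load, and post-init fires once all three are present.
; Session, network and travel errors destroy the session and show a dialog that stores the prior state.
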(event Custom|GIE%20Update%20GI%20State
  (params (PlayerState :type AE_PlayerState%20Enum :default "NewEnumerator0"))
  ;[1 1 1] Update: GI State to Player State
  (if (!= (Variables|AppData|GetGIState) (Utilities|Enum|LiteralenumAE_PlayerState "NewEnumerator1")) ; Only update GiState with PlayerState\nwhen GiState != MainMenu
    (CallFunction|GISetPlayerState PlayerState)))

(event Custom|GIE%20Register%20PS
  (params (PlayerStateRef :type BG%20Player%20State%20Object%20Reference))
  ;[1 1 1] Level Load: Register New Objects
  (Variables|ObjectReference|SetPlayerStateRef PlayerStateRef)
  (CallFunction|GICheckPostInit))

(event Custom|GIE%20Register%20PLC
  (params (PlyrCtrlRef :type BC%20Ctrl%20Player%20Object%20Reference))
  ;[1 1 1] Level Load: Register New Objects
  (Variables|ObjectReference|SetPlayerControlRef PlyrCtrlRef)
  (CallFunction|GICheckPostInit))

(event Custom|GIE%20Register%20MAP
  ;[1 1 1] Level Load: Register New Objects
  (Variables|FlowControl|SetTMapLoaded true)
  (CallFunction|GICheckPostInit))

(event Custom|GIE%20Start%20Host%20Game
  (params (GameDetails :type AS%20Game%20Details%20Structure) (PlayerList :type Array%20of%20AS%20Player%20Details%20Structures))
  ;[1 1 1] Start/Continue a campaign
  ; Host/Join/Destroy an Online Game
  (CallFunction|GISetGameDetails GameDetails)
  (CallFunction|GISetPlayerList PlayerList)
  (|Session (Game|GetPlayerController 0) (.NumPlyrPlyrs (Utilities|Struct|BreakAS_GameDetails GameDetails)) (Variables|FlowControl|GetTLanEnabled)
    (:OnSuccess
      (bind _retval (CallFunction|GISetPlayerState "NewEnumerator12"))
      (if (== (Utilities|Enum|LiteralenumAE_XReturnValues "NewEnumerator0") _retval)
        (Variables|FlowControl|SetTIsHost true)
        (CallFunction|GIShowMainMenu "NewEnumerator16")
        (CallFunction|GIResetPostInit)
        (Game|OpenLevel(byName) "Map3_Landscape" true "listen")
        (else
          (Variables|Temp|SetTmpBool false))))
    (:OnFailure
      (CallFunction|EventSessionError "Sorry, Failed to create session"))))

(event Custom|Event%20Session%20Error
  (params (ErrorStr :type String))
  ;[1 1 1] Network Error Events
  (CallFunction|GIShowErrorDialog "Session Error Event" ErrorStr))

(event Custom|GIE%20Start%20Campaign
  (params (StartType :type Integer :default 0) (LoadId :type Integer :default 0))
  ;[1 1 1] Start/Continue a campaign
  ; Host/Join/Destroy an Online Game
  (CallFunction|GILoadCampaignDetails StartType LoadId)
  (CallFunction|GISetPlayerState "NewEnumerator12")
  (CallFunction|GIShowMainMenu "NewEnumerator16")
  (CallFunction|GIResetPostInit)
  (Game|OpenLevel(byName) (Variables|GameData|GetGameMap) true "listen"))

(event Custom|DestroySessionCaller
  ;[1 1 1] Start/Continue a campaign
  ; Host/Join/Destroy an Online Game
  (|DestroySession (Game|GetPlayerController 0)))

(event Custom|GIE%20Join%20Game
  (params (Session :type Blueprint%20Session%20Result%20Structure))
  ;[1 1 1] Start/Continue a campaign
  ; Host/Join/Destroy an Online Game
  (|JoinSession (Game|GetPlayerController 0) Session
    (:OnSuccess
      (bind _retval (CallFunction|GISetPlayerState "NewEnumerator12"))
      (if (== (Utilities|Enum|LiteralenumAE_XReturnValues "NewEnumerator0") _retval)
        (CallFunction|GIShowMainMenu "NewEnumerator16")
        (else
          (Variables|Temp|SetTmpBool false))))
    (:OnFailure
      (CallFunction|EventSessionError "Sorry, Failed to join session"))))

(event Custom|Show%20Main%20Menu
  (params (MenuScreen :type AE_MenuScreens%20Enum))
  ;[1 1 1] Show Main Menus
  (CallFunction|GIShowMainMenu MenuScreen))

(event EventHandleNetworkError
  (params (FailureType :type ENetworkFailure%20Enum :default "NetDriverAlreadyExists") (bIsServer :type Boolean))
  ;[1 1 1] Network Error Events
  (CallFunction|GIShowErrorDialog "Network Error Event" (Utilities|String|EnumtoString FailureType)))

(event EventHandleTravelError
  (params (FailureType :type ETravelFailure%20Enum :default "NoLevel"))
  ;[1 1 1] Network Error Events
  (CallFunction|GIShowErrorDialog "Travel Error Event" (Utilities|String|EnumtoString FailureType)))

(fn GICheckPostInit
  ;[1 1 1] If:     All Object References are Valid
  ; Set: TPostInit = True
  (Utilities|IsValid (Variables|ObjectReference|GetPlayerControlRef)
    (:Is%20Valid
      (Utilities|IsValid (Variables|ObjectReference|GetPlayerStateRef)
        (:Is%20Valid
          (if (Variables|FlowControl|GetTMapLoaded)
            (Variables|FlowControl|SetTPostInit true)
            (Default|PSSetPostInit (Variables|ObjectReference|GetPlayerStateRef))))))))

(fn GISetPlayerState
  (params (NewState :type AE_PlayerState%20Enum))
  (Utilities|IfDbgPrnt
    (:ExecDbg
      (Variables|Temp|SetTmpStr1 (Utilities|String|EnumtoString (Variables|AppData|GetGIState)))
      (Variables|Temp|SetTmpStr2 (Utilities|String|EnumtoString NewState))
      (Variables|Temp|SetTmpBool false))
    (:ExecFinish
      (if (== (Variables|AppData|GetGIState) NewState)
        ;[1 1 1] Hide whatever menu widget was associated with previous state
        (Development|PrintString (Utilities|String|ToString(Text) (Utilities|Text|FormatText "Error: trying to reenter same state: {State}" (Utilities|Text|ToText(String) (Utilities|String|EnumtoString (Variables|AppData|GetGIState))))))
        (LocalVariables|SetLclRetVal (Utilities|Enum|LiteralenumAE_XReturnValues "NewEnumerator4"))
        (else
          (switch Utilities|FlowControl|Switch|SwitchonAE_PlayerState (Variables|AppData|GetGIState)
            (:NewEnumerator0
              _)
            (:NewEnumerator1
              (Widget|RemovefromParent (Variables|Menus|GetMenuFrontPage)))
            (:NewEnumerator2
              (Widget|RemovefromParent (Variables|Menus|GetMenuNetworkLobby)))
            (:NewEnumerator12
              _)
            (:NewEnumerator13
              _)
            (:NewEnumerator21
              (Widget|RemovefromParent (Variables|Menus|GetMenuLoadScreen) :!label _label))
            (:NewEnumerator14
              (goto _label))
            (:NewEnumerator16
              _)
            (:NewEnumerator4
              (Widget|RemovefromParent (Variables|Menus|GetMenuErrorDialog))))
          (bind _output_get (Variables|AppData|SetGIState NewState))
          (LocalVariables|SetLclRetVal (Utilities|Enum|LiteralenumAE_XReturnValues "NewEnumerator0"))))
      (return _output_get (LocalVariables|GetLclRetVal)))))

(fn GIShowMainMenu
  (params (NewMenu :type AE_MenuScreens%20Enum))
  (bind _returnvalue (Game|GetPlayerController 0))
  (bind _returnvalue_2 (Game|GetPlayerController 0))
  (bind _returnvalue_3 (Game|GetPlayerController 0))
  (bind _returnvalue_4 (Game|GetPlayerController 0))
  (bind _returnvalue_5 (Game|GetPlayerController 0))
  (bind _returnvalue_6 (Game|GetPlayerController 0))
  (bind _returnvalue_7 (Game|GetPlayerController 0))
  (bind _returnvalue_8 (Game|GetPlayerController 0))
  (bind _returnvalue_9 (Game|GetPlayerController 0))
  (bind _gistatepreerror (Variables|AppData|GetGIStatePreError))
  (Variables|Menus|SetMenuPrevious (Variables|Menus|GetMenuNow))
  (Variables|Menus|SetGenWidgetPrevRef (Variables|Menus|GetGenWidgetNowRef))
  (Variables|Menus|SetMenuNow NewMenu)
  (Utilities|IfDbgPrnt
    (:ExecDbg
      (Variables|Temp|SetTmpStr (Utilities|String|EnumtoString (Variables|AppData|GetGIState)))
      (if (Utilities|Enum|Equal(Enum) (Variables|AppData|GetGIState) "NewEnumerator4")
        (bind _output_get (Variables|AppData|SetGIState _gistatepreerror))
        (Variables|Temp|SetTmpStr1 (Utilities|String|EnumtoString _gistatepreerror))
        (Variables|Temp|SetTmpStr2 (Utilities|String|EnumtoString _output_get))))
    (:ExecFinish
      (Utilities|FlowControl|Sequence
        (:then_0
          ;[1 1 1] Open Main Menu Level and set GIState to Main Menu if necessary
          (if (and (Utilities|Enum|NotEqual(Enum) (Variables|Menus|GetMenuNow) "NewEnumerator7") (Math|Boolean|ORBoolean (Utilities|Enum|Equal(Enum) (Variables|AppData|GetGIState) "NewEnumerator0") (Utilities|Enum|Equal(Enum) (Variables|AppData|GetGIState) "NewEnumerator1") (Utilities|Enum|Equal(Enum) (Variables|AppData|GetGIState) "NewEnumerator2") (Utilities|Enum|Equal(Enum) (Variables|AppData|GetGIState) "NewEnumerator8"))) ; If NOT currently in a main menu state\nOpen Main Menu level
            _
            (else
              (Game|OpenLevel(byName) "MainMenu" true "listen")))
          (if (and (Utilities|Enum|Equal(Enum) (Variables|Menus|GetMenuNow) "NewEnumerator5") (Utilities|Enum|NotEqual(Enum) (Variables|AppData|GetGIState) "NewEnumerator2"))
            (CallFunction|GISetPlayerState "NewEnumerator2")
            (elif (and (Utilities|Enum|NotEqual(Enum) (Variables|Menus|GetMenuNow) "NewEnumerator7") (Utilities|Enum|NotEqual(Enum) (Variables|AppData|GetGIState) "NewEnumerator1"))
              (CallFunction|GISetPlayerState "NewEnumerator1"))))
        (:then_1
          (switch Utilities|FlowControl|Switch|SwitchonAE_MenuScreens (Variables|Menus|GetMenuNow)
            (:NewEnumerator0
              ;[1 1 1] Show: Main Menu (called from MainMenu level start)
              (Utilities|IsValid (Variables|Menus|GetMenuFrontPage)
                (:Is%20Valid
                  _)
                (:Is%20Not%20Valid
                  (bind _returnvalue_10 (UserInterface|CreateWidget "/Game/Blueprints/Widgets/BU_MMFrontPage.BU_MMFrontPage_C" _returnvalue_2))
                  (bind _output_get_2 (Variables|Menus|SetMenuFrontPage _returnvalue_10))))
              (Variables|Menus|SetGenWidgetNowRef _output_get_2)
              (Input|SetInputModeUIOnly _returnvalue_2 _output_get_2 false)
              (UserInterface|Viewport|AddtoViewport _output_get_2 0))
            (:NewEnumerator1
              ;[1 1 1] Campaign New
              (Utilities|IsValid (Variables|Menus|GetMenuCpgnNew)
                (:Is%20Valid
                  _)
                (:Is%20Not%20Valid
                  (bind _returnvalue_11 (UserInterface|CreateWidget "/Game/Blueprints/Widgets/BU_MMCpgnNew.BU_MMCpgnNew_C" _returnvalue_3))
                  (bind _output_get_3 (Variables|Menus|SetMenuCpgnNew _returnvalue_11))))
              (Variables|Menus|SetGenWidgetNowRef _output_get_3)
              (Input|SetInputModeUIOnly _returnvalue_3 _output_get_3 false)
              (UserInterface|Viewport|AddtoViewport _output_get_3 0))
            (:NewEnumerator2
              ;[1 1 1] Campaign Front Page
              (Utilities|IsValid (Variables|Menus|GetMenuCpgnFrontPage)
                (:Is%20Valid
                  _)
                (:Is%20Not%20Valid
                  (bind _returnvalue_12 (UserInterface|CreateWidget "/Game/Blueprints/Widgets/BU_MMCpgnFrontPage.BU_MMCpgnFrontPage_C" _returnvalue_7))
                  (bind _output_get_4 (Variables|Menus|SetMenuCpgnFrontPage _returnvalue_12))))
              (Variables|Menus|SetGenWidgetNowRef _output_get_4)
              (Input|SetInputModeUIOnly _returnvalue_7 _output_get_4 false)
              (UserInterface|Viewport|AddtoViewport _output_get_4 0))
            (:NewEnumerator4
              ;[1 1 1] Campaign Front Page
              (Utilities|IsValid (Variables|Menus|GetMenuCpgnSkmshNew)
                (:Is%20Valid
                  _)
                (:Is%20Not%20Valid
                  (bind _returnvalue_13 (UserInterface|CreateWidget "/Game/Blueprints/Widgets/BU_MMCpgnSkmsh.BU_MMCpgnSkmsh_C" _returnvalue_4))
                  (bind _output_get_5 (Variables|Menus|SetMenuCpgnSkmshNew _returnvalue_13))))
              (Variables|Menus|SetGenWidgetNowRef _output_get_5)
              (Input|SetInputModeUIOnly _returnvalue_4 _output_get_5 false)
              (UserInterface|Viewport|AddtoViewport _output_get_5 0))
            (:NewEnumerator5
              ;[1 1 1] Network Lobby
              (Utilities|IsValid (Variables|Menus|GetMenuNetworkLobby)
                (:Is%20Valid
                  _)
                (:Is%20Not%20Valid
                  (bind _returnvalue_14 (UserInterface|CreateWidget "/Game/Blueprints/Widgets/BU_MMNetworkLobby.BU_MMNetworkLobby_C" _returnvalue))
                  (bind _output_get_6 (Variables|Menus|SetMenuNetworkLobby _returnvalue_14))))
              (Variables|Menus|SetGenWidgetNowRef _output_get_6)
              (Input|SetInputModeUIOnly _returnvalue _output_get_6 false)
              (UserInterface|Viewport|AddtoViewport _output_get_6 0))
            (:NewEnumerator6
              ;[1 1 1] Skirmish Start
              (Utilities|IsValid (Variables|Menus|GetMenuSkrmshNew)
                (:Is%20Valid
                  _)
                (:Is%20Not%20Valid
                  (UserInterface|CreateWidget "/Game/Blueprints/Widgets/BU_MMCpgnFrontPage.BU_MMCpgnFrontPage_C" _returnvalue_8)
                  (bind _output_get_7 (Variables|Menus|SetMenuSkrmshNew 0))))
              (Variables|Menus|SetGenWidgetNowRef _output_get_7)
              (Input|SetInputModeUIOnly _returnvalue_8 _output_get_7 false)
              (UserInterface|Viewport|AddtoViewport _output_get_7 0))
            (:NewEnumerator9
              ;[1 1 1] Army Builder
              (Utilities|IsValid (Variables|Menus|GetMenuArmyBuiler)
                (:Is%20Valid
                  _)
                (:Is%20Not%20Valid
                  (UserInterface|CreateWidget "/Game/Blueprints/Widgets/BU_MMArmyBuilder.BU_MMArmyBuilder_C" _returnvalue_5)
                  (bind _output_get_8 (Variables|Menus|SetMenuArmyBuiler 0))))
              (Variables|Menus|SetGenWidgetNowRef _output_get_8)
              (Input|SetInputModeUIOnly _returnvalue_5 _output_get_8 false)
              (UserInterface|Viewport|AddtoViewport _output_get_8 0))
            (:NewEnumerator10
              ;[1 1 1] Barracks
              (Utilities|IsValid (Variables|Menus|GetMenuBarracks)
                (:Is%20Valid
                  _)
                (:Is%20Not%20Valid
                  (bind _returnvalue_15 (UserInterface|CreateWidget "/Game/Blueprints/Widgets/BU_MMBarracks.BU_MMBarracks_C" _returnvalue_6))
                  (bind _output_get_9 (Variables|Menus|SetMenuBarracks _returnvalue_15))))
              (Variables|Menus|SetGenWidgetNowRef _output_get_9)
              (Input|SetInputModeUIOnly _returnvalue_6 _output_get_9 false)
              (UserInterface|Viewport|AddtoViewport _output_get_9 0))
            (:NewEnumerator16
              ;[1 1 1] Load Screen
              (Utilities|IsValid (Variables|Menus|GetMenuLoadScreen)
                (:Is%20Valid
                  _)
                (:Is%20Not%20Valid
                  (bind _returnvalue_16 (UserInterface|CreateWidget "/Game/Blueprints/Widgets/BU_MMLoadScreen.BU_MMLoadScreen_C" _returnvalue_9))
                  (bind _output_get_10 (Variables|Menus|SetMenuLoadScreen _returnvalue_16))))
              (Variables|Menus|SetGenWidgetNowRef 0)
              (Input|SetInputModeUIOnly _returnvalue_9 _output_get_10 false)
              (UserInterface|Viewport|AddtoViewport _output_get_10 0))))
        (:then_2
          (Widget|SetVisibility (Variables|Menus|GetGenWidgetNowRef) "Visible")
          (if (!= (Variables|Menus|GetGenWidgetNowRef) (Variables|Menus|GetGenWidgetPrevRef))
            (Widget|SetVisibility (Variables|Menus|GetGenWidgetPrevRef) "Hidden")))))))

(fn GIShowErrorDialog
  (params (Error%20Class :type String) (Error%20Reason :type String))
  (bind _returnvalue (Utilities|Text|ToText(String) Error%20Class))
  (bind _returnvalue_2 (Utilities|Text|ToText(String) Error%20Reason))
  (bind _gistate (Variables|AppData|GetGIState))
  (if (Networking|IsServer)
    (LocalVariables|SetLclServerStr "Host")
    (else
      (LocalVariables|SetLclServerStr "Client")))
  (bind _output_get (LocalVariables|SetLclDbgOpStr (Utilities|String|ToString(Text) (Utilities|Text|FormatText "===== ERROR [{server} >  BG_GameInst > Event Graph > {type}]-- {reason}" (Utilities|Text|ToText(String) (LocalVariables|GetLclServerStr)) _returnvalue _returnvalue_2))))
  (Development|PrintString _output_get)
  (LocalVariables|SetLclUserOpStr (Utilities|String|ToString(Text) (Utilities|Text|FormatText "Sorry, there was a {type} on your {server} -- {reason}" _returnvalue (Utilities|Text|ToText(String) (LocalVariables|GetLclServerStr)) _returnvalue_2)))
  (if (Utilities|Enum|NotEqual(Enum) _gistate "NewEnumerator4")
    (Variables|AppData|SetGIStatePreError _gistate))
  (bind _retval (CallFunction|GISetPlayerState "NewEnumerator4"))
  (if (== (Utilities|Enum|LiteralenumAE_XReturnValues "NewEnumerator0") _retval)
    (CallFunction|DestroySessionCaller)
    (Utilities|IsValid (Variables|Menus|GetMenuErrorDialog)
      (:Is%20Valid
        _)
      (:Is%20Not%20Valid
        (bind _returnvalue_3 (UserInterface|CreateWidget "/Game/Blueprints/Widgets/BU_ErrorDialog.BU_ErrorDialog_C"))
        (Variables|Menus|SetMenuErrorDialog _returnvalue_3)))
    (Default|SetMessage (Variables|Menus|GetMenuErrorDialog) (LocalVariables|GetLclUserOpStr) (Variables|AppData|GetGIStatePreError))
    (UserInterface|Viewport|AddtoViewport (Variables|Menus|GetMenuErrorDialog) 0)
    (Input|SetInputModeUIOnly (Game|GetPlayerController 0) (Variables|Menus|GetMenuErrorDialog) false)
    (else
      (Variables|Temp|SetTmpBool false))))

(fn GISetGameDetails
  (params (Game%20Details :type AS%20Game%20Details%20Structure))
  (Variables|GameData|SetGameDetails Game%20Details))

(fn GIGetGameDetails
  (bind _gamedetails (Variables|GameData|GetGameDetails))
  (bind (_gametype _numplyrplyrs _numcpuplyrs _map) (Utilities|Struct|BreakAS_GameDetails _gamedetails))
  (return _gametype _numplyrplyrs _numcpuplyrs _map))

(fn GISetPlayerList
  (params (PlayerList :type Array%20of%20AS%20Player%20Details%20Structures))
  (Variables|PlayerData|SetPlayerList PlayerList))

(fn GIGetPlayerList
  (return (Variables|PlayerData|GetPlayerList)))

(fn GILoadCampaignDetails
  (params (StartType :type Integer) (LoadId :type Integer))
  (Variables|GameData|SetGameMap (Utilities|Array|Get(acopy) (Variables|GameData|GetGameMapNames)))
  (Variables|PlayerData|SetPlayerDetails (Utilities|Struct|MakeAS_PlayerDetails 0 "NewEnumerator0" "NewEnumerator0" "NewEnumerator0" "NewEnumerator0" 1))
  (Variables|GameData|SetGameDetails (Utilities|Struct|MakeAS_GameDetails "NewEnumerator3" 1 1 (Variables|GameData|GetGameMap)))
  (return))

(fn GIResetPostInit
  (Variables|ObjectReference|SetPlayerControlRef (Variables|ObjectReference|GetNullPlayerControlRef))
  (Variables|ObjectReference|SetPlayerStateRef (Variables|ObjectReference|GetNullPlayerStateRef))
  (Variables|FlowControl|SetTMapLoaded false)
  (Variables|FlowControl|SetTPostInit false))

(fn GIInit
  (Variables|GameData|SetGameMapNames (Utilities|Array|MakeArray "Map3_Landscape" "Map5_Large")))