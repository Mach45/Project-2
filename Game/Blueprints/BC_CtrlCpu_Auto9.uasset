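; BC_CtrlCpu_Auto9 is a CPU player controller that takes part in the game's join and start-of-play handshake.
; It caches the game mode and instance; on joining, it stores game and player details and spawns character and skill library actors.
; Once all have joined, it reports a new player state to the game mode, then flags play start on notification.
; AICInit is empty and unit-controller spawning is disconnected; AICSetGameControl receives those references instead.
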(event `self.ReceiveBeginPlay`
  ;[1 1 1] Begin Play
  (bind _asbg_game_mode (cast `/Game/Blueprints/Game/BG_GameMode` (`GameplayStatics.GetGameMode`))
    (:`then`
      (set `self.GameMode` _asbg_game_mode)
      (bind _asbg_game_instance (cast `/Game/Blueprints/Game/BG_GameInstance` (`GameplayStatics.GetGameInstance`))
        (:`then`
          (set `self.GameInstance` _asbg_game_instance))
        (:`CastFailed`
          (`KismetSystemLibrary.PrintString` "##### ERROR  [BC_PlyrCpu > EventGraph] -- Set Game Instance failed"))))
    (:`CastFailed`
      (`KismetSystemLibrary.PrintString` "##### ERROR  [BC_PlyrAi > EventGraph] -- GameMode get failed"))))

(event `AIC Post Joined`
  (params (`Game Details` :type "/Game/Blueprints/Structs/AS_GameDetails Structure") (`Player Details` :type "/Game/Blueprints/Structs/AS_PlayerDetails Structure"))
  (`self.AIC Setup Joined` `Game Details` `Player Details`))

(event `AIC All Joined Ntf`
  (params (PlayerList :type "Array of /Game/Blueprints/Structs/AS_PlayerDetails Structure"))
  (set `self.PlayerList` PlayerList)
  (`/Game/Blueprints/Game/BG_GameMode.RPC GM Update Player State` (`self.GameMode`) (`.PlayerId_43_A122F5E64CD684113AA80584C92C8D0F` (break `/Game/Blueprints/Structs/AS_PlayerDetails` (`self.Player Details`))) "NewEnumerator21"))

(event `AIC All Start Plying Ntf`
  (set `self.TPlayStarted` true))

(fn `AIC Init`
  (params (PlayerId :type Integer :default 0) (PlayerRace :type "/Game/Blueprints/Enums/AE_CharRace Enum" :default "NewEnumerator0") (PlayerClass :type "/Game/Blueprints/Enums/AE_CharClass Enum" :default "NewEnumerator8") (StartLoc :type "Transform Structure") (MusterLoc :type "Vector Structure" :default (0.0 0.0 0.0)) (ResourceLocs :type "Array of /Game/Blueprints/Actors/BA_ResourcePoint Object Reference")))

(fn `AIC Set Game Control`
  (params (GameCtrlRef :type "/Game/Blueprints/BC_GameControl Object Reference") (UnitCtrlRef :type "/Game/Blueprints/BC_CtrlUnit Object Reference"))
  (set `self.GameControl` GameCtrlRef)
  (set `self.UnitControl` UnitCtrlRef))

(fn `AIC Setup Joined`
  (params (GameDetails :type "/Game/Blueprints/Structs/AS_GameDetails Structure") (PlayerDetails :type "/Game/Blueprints/Structs/AS_PlayerDetails Structure"))
  (set `self.Game Details` GameDetails)
  (set `self.Player Details` PlayerDetails)
  (bind _asbg_game_mode (cast `/Game/Blueprints/Game/BG_GameMode` (`GameplayStatics.GetGameMode`))
    (:`then`
      (set `self.GameMode` _asbg_game_mode)
      (`|ExecutionSequence`
        (:`then_0`
          ;[1 1 1] Create: Character & Skill Libraries - remove
          (bind _returnvalue (`|SpawnActorFromClass` "/Game/Blueprints/Game/BP_LibCharacters.BP_LibCharacters_C" (`self.TmpTransform`) "AlwaysSpawn" "OverrideRootScale"))
          (set `self.CharsLib` _returnvalue)
          (if (not (`KismetSystemLibrary.IsValid` _returnvalue))
            (`KismetSystemLibrary.PrintString` "##### ERROR [BPG_MyController:PLCInitPlayer] -- Char Lib not Instantiated")))
        (:`then_1`
          (bind _returnvalue_2 (`|SpawnActorFromClass` "/Game/Blueprints/Game/BP_LibSkills.BP_LibSkills_C" (`self.TmpTransform`) "AlwaysSpawn" "OverrideRootScale"))
          (set `self.SkillsLib` _returnvalue_2)
          (if (not (`KismetSystemLibrary.IsValid` _returnvalue_2))
            (`KismetSystemLibrary.PrintString` "##### ERROR  [BPG_MyController:PLCInitPlayer] -- Skill Lib not Instantiated")))))
    (:`CastFailed`
      (`KismetSystemLibrary.PrintString` "##### ERROR  [BC_PlyrAi > EventGraph] -- GameMode get failed"))))

(fn `UserConstructionScript`)